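; Player character for a hover game: a twin-thruster craft flying in the XZ plane, scoring over time and for full-rotation flips.
; While unpaused, Tick turns left/right input into decaying power that drives rotation and thrust against gravity, integrated by hand.
; Power also feeds thruster particle parameters, and with distance from spawn drives post-process intensities.
; A turn state machine tints the material and awards flips; leaving bounds spawns a death effect and resets.
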(event `self.ReceiveBeginPlay`
  (bind _returnvalue (`PrimitiveComponent.CreateDynamicMaterialInstance` (`self.Cube8`) 0 "/Game/VFXCollections/Hover/Materials/M_UnlitColor_Inst.M_UnlitColor_Inst" "None"))
  (set `self.MyColor` _returnvalue)
  (set `self.OritinalTransform` (`KismetMathLibrary.MakeTransform` (`self.K2_GetActorLocation`) (`self.K2_GetActorRotation`) (`self.GetActorScale3D`)))
  (bind _outactors (`GameplayStatics.GetAllActorsOfClass` "/Script/Engine.PostProcessVolume"))
  (bind _output (`|GetArrayItem` _outactors))
  (`/Engine/EditorBlueprintResources/StandardMacros.IsValid` _output
    (:`Is Valid`
      (set `self.PostProcess` _output))))

(event `self.ReceiveTick`
  (params (DeltaSeconds :type "Float (single-precision)"))
  (bind _returnvalue (* (`self.radian`) -1.0))
  (bind _returnvalue_2 (`KismetMathLibrary.MakeVector` (* (`KismetMathLibrary.Sin` _returnvalue) 200.0) 0.0 (* (`KismetMathLibrary.Cos` _returnvalue) 200.0)))
  (`/Engine/EditorBlueprintResources/StandardMacros.Gate` false :!label _label
    (:`Exit`
      (`self.UpdateTurn`)
      (`self.CalculateScore`)
      (`NiagaraComponent.SetVariableFloat` (`self.ThrusterSystem_r`) "SpawnRate" (* (`self.power_r`) (`self.PARITLC_MULTIPLY`)))
      (`NiagaraComponent.SetVariableFloat` (`self.ThrusterSystem_l`) "SpawnRate" (* (`self.power_l`) (`self.PARITLC_MULTIPLY`)))
      (`NiagaraComponent.SetVariableFloat` (`self.ThrusterSystem_l`) "LerpFireZeroToOne" (`KismetMathLibrary.Abs` (- (`self.power_r`) (`self.power_l`))))
      (`NiagaraComponent.SetVariableFloat` (`self.ThrusterSystem_r`) "LerpFireZeroToOne" (`KismetMathLibrary.Abs` (- (`self.power_r`) (`self.power_l`))))
      (`self.UpdatePostProcess`)
      (`self.CheckGameOver`)
      ;[1 1 1] Comment
      (set `self.power_l` (`KismetMathLibrary.FMax` (- (`self.power_l`) (* (`self.POWER_DECAY`) DeltaSeconds))))
      ;[1 1 1] Comment
      (set `self.power_r` (`KismetMathLibrary.FMax` (- (`self.power_r`) (* (`self.POWER_DECAY`) DeltaSeconds))))
      ;[1 1 1] Comment
      (set `self.power_r` (`KismetMathLibrary.FMin` (+ (`self.power_r`) (* DeltaSeconds (`self.POWER_DELTA`) (`self.GetInputAxisValue`))) (`self.POWER_MAX`)))
      ;[1 1 1] Comment
      (set `self.power_l` (`KismetMathLibrary.FMin` (+ (`self.power_l`) (* DeltaSeconds (`self.POWER_DELTA`) (`self.GetInputAxisValue`))) (`self.POWER_MAX`)))
      (set `self.Velocity` (+ (`self.Velocity`) (* (`self.Gravity`) DeltaSeconds)))
      (set `self.radVel` (+ (* (`self.radVel`) 0.95) (* (- (`self.power_l`) (`self.power_r`)) (`self.RAD_DELTA`) DeltaSeconds)))
      (set `self.radian` (+ (`self.radian`) (`self.radVel`)))
      (`self.K2_SetActorRotation` (`KismetMathLibrary.MakeRotFromXZ` (`KismetMathLibrary.MakeVector` 0.0 1.0) _returnvalue_2))
      (set `self.Acceleration` _returnvalue_2)
      (set `self.Velocity` (+ (`self.Velocity`) (* (`self.Acceleration`) (* DeltaSeconds (`self.ACC_MULTIPLY`) (`self.ACC_MULTIPLY`) (+ (`KismetMathLibrary.Abs` (`self.power_r`)) (`KismetMathLibrary.Abs` (`self.power_l`)))))))
      (`self.K2_SetActorLocation` (+ (`self.K2_GetActorLocation`) (* (`self.Velocity`) DeltaSeconds))))))

(event `Pause`
  (goto _label :!via `Close`))

(event `Resume`
  (goto _label :!via `Open`))

(event `UpdatePostProcess`
  (bind _postprocess (`self.PostProcess`))
  (`/Engine/EditorBlueprintResources/StandardMacros.IsValid` (`self.PostProcess`)
    (:`Is Valid`
      (bind _structout (setmembers `PostProcessSettings` :`StructRef` (`PostProcessVolume.Settings` _postprocess) :`SceneFringeIntensity` (* (`KismetMathLibrary.Abs` (- (`self.power_r`) (`self.power_l`))) 2.0) :`LensFlareIntensity` (/ (`KismetMathLibrary.MultiplyMultiply_FloatFloat` (`KismetMathLibrary.Vector_Distance` (.location (`self.OritinalTransform`)) (`self.K2_GetActorLocation`)) 2.0) 60000.0) :`VignetteIntensity` 0.4))
      (set `PostProcessVolume.Settings` _structout _postprocess))))

(event `CheckGameOver`
  ;[1 1 1] Game Over
  (if (> (`KismetMathLibrary.FMax` (`KismetMathLibrary.Abs` (.x (`self.K2_GetActorLocation`))) (`KismetMathLibrary.Abs` (.z (`self.K2_GetActorLocation`)))) 3000.0)
    ;[1 1 1] Comment
    (`NiagaraFunctionLibrary.SpawnSystemAtLocation` "/Game/VFXCollections/Hover/Effects/PlayerDeadSystem.PlayerDeadSystem" (`KismetMathLibrary.MakeVector` (`KismetMathLibrary.FClamp` (.x (`self.K2_GetActorLocation`)) -2000.0 2000.0) (.y (`self.K2_GetActorLocation`)) (`KismetMathLibrary.FClamp` (.z (`self.K2_GetActorLocation`)) -1000.0 1000.0)) (struct) (`KismetMathLibrary.Conv_DoubleToVector` 10.0))
    (`self.Reset`)))

(event `Reset`
  (set `self.Velocity` (0.0 0.0 0.0))
  (set `self.Acceleration` (0.0 0.0 0.0))
  (`self.K2_SetActorTransform` (`self.OritinalTransform`))
  (set `self.radian` 0.0)
  (set `self.Score` 0)
  (set `self.TurnState` "NewEnumerator0"))

(event `UpdateTurn`
  (bind _returnvalue (mod (`KismetMathLibrary.RadiansToDegrees` (`self.radian`)) 360.0))
  (`MaterialInstanceDynamic.SetVectorParameterValue` (`self.MyColor`) "Color" (`KismetMathLibrary.SelectColor` (struct :`R` 0.182292 :`G` 0.173643 :`B` 0.157974 :`A` 1.0) (struct :`R` 1.0 :`G` 0.033409 :`A` 1.0) (== (`self.TurnState`) 0)))
  (switch `/Game/VFXCollections/Hover/Blueprints/TurnState` (`self.TurnState`)
    (:`NewEnumerator0`
      (if (> (`KismetMathLibrary.Abs` _returnvalue) 40.0)
        (set `self.TurnState` "NewEnumerator1")
        (set `self.TurnStartDegree` _returnvalue)))
    (:`NewEnumerator1`
      (if (< (`KismetMathLibrary.Abs` (mod (`KismetMathLibrary.RadiansToDegrees` (`self.radian`)) 360.0)) 30.0)
        (set `self.TurnState` "NewEnumerator0")
        (elif (> (`KismetMathLibrary.Abs` (mod (`KismetMathLibrary.RadiansToDegrees` (`self.radian`)) 360.0)) 350.0)
          (set `self.Score` (+ (`self.Score`) 500))
          (set `self.TurnState` "NewEnumerator0")
          (`NiagaraFunctionLibrary.SpawnSystemAtLocation` "/Game/VFXCollections/Hover/Effects/TurnSuccessSystem.TurnSuccessSystem" (`self.K2_GetActorLocation`))
          (if (> (mod (`KismetMathLibrary.RadiansToDegrees` (`self.radian`)) 360.0) 0.0)
            (set `self.radian` (`KismetMathLibrary.DegreesToRadians` (* (- 360.0 (mod (`KismetMathLibrary.RadiansToDegrees` (`self.radian`)) 360.0)) -1.0)))
            (else
              (set `self.radian` (`KismetMathLibrary.DegreesToRadians` (+ 360.0 (mod (`KismetMathLibrary.RadiansToDegrees` (`self.radian`)) 360.0)))))))))))

(event `CalculateScore`
  (set `self.Score` (+ (`self.Score`) 1)))

(fn `UserConstructionScript`)