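; BP_Particle is an actor that acts as a single sphere particle, moving and changing opacity over a limited lifetime.
; On BeginPlay it puts a dynamic instance of M_BPParticle on its Sphere.
; Each Tick it integrates acceleration into velocity and velocity into location without sweeping, then sets material Opacity from a float curve sampled at normalized age.
; It destroys itself once its age exceeds its lifetime.
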(event `self.ReceiveBeginPlay`
  (bind _returnvalue (`KismetMaterialLibrary.CreateDynamicMaterialInstance` "/Game/VFXCollections/BPParticle/M_BPParticle.M_BPParticle"))
  (bind _output_get (set `self.Material` _returnvalue))
  (`PrimitiveComponent.SetMaterial` (`self.Sphere`) 0 _output_get))

(event `self.ReceiveTick`
  (params (DeltaSeconds :type "Float (single-precision)"))
  (bind _output_get (set `self.Age` (+ (`self.Age`) DeltaSeconds)))
  (if (> _output_get (`self.Lifetime`))
    (`self.K2_DestroyActor`)
    (else
      (set `self.Velocity` (+ (`self.Velocity`) (* (`self.Acceleration`) DeltaSeconds)))
      (`self.K2_SetActorLocation` (+ (`self.K2_GetActorLocation`) (* (`self.Velocity`) DeltaSeconds)))
      (`MaterialInstanceDynamic.SetScalarParameterValue` (`self.Material`) "Opacity" (`CurveFloat.GetFloatValue` (`self.Curve`) (/ (`self.Age`) (`self.Lifetime`)))))))

(fn `UserConstructionScript`)