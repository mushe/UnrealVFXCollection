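; BP_ParticleEmitter is an actor that emits bursts of BP_Particle actors as a Blueprint-driven particle effect.
; Its Burst event spawns particles in a loop driven by BurstRate, at the emitter's location with a configurable uniform scale.
; Each particle receives a random-direction velocity and a lifetime, with speed and lifetime drawn from min/max ranges.
; BeginPlay and the construction script are empty, so nothing here triggers a burst automatically.
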(event `Burst`
  (for _ (range (+ (`self.BurstRate`) 1))
    (bind _returnvalue (`|SpawnActorFromClass` "/Game/VFXCollections/BPParticle/BP_Particle.BP_Particle_C" (`KismetMathLibrary.MakeTransform` (`self.K2_GetActorLocation`) (struct) (`KismetMathLibrary.Conv_DoubleToVector` (`self.Scale`))) "Undefined" "OverrideRootScale" null null))
    (set `/Game/VFXCollections/BPParticle/BP_Particle.Velocity` (* (`KismetMathLibrary.RandomUnitVector`) (`KismetMathLibrary.RandomFloatInRange` (`self.SpeedMin`) (`self.SpeedMax`))) _returnvalue)
    (set `/Game/VFXCollections/BPParticle/BP_Particle.Lifetime` (`KismetMathLibrary.RandomFloatInRange` (`self.LifetimeMin`) (`self.LifetimeMax`)) _returnvalue)))

(event `self.ReceiveBeginPlay`)

(fn `UserConstructionScript`)